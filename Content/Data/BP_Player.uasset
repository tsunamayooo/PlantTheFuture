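; Player pawn for an on-rails shooter with mouse look outside VR, riding a chain of splines.
; Tick advances it along the current spline, scaling mouse-button-controlled speed by pitch, so descents accelerate and climbs slow.
; Holding Fire spawns balls while ammo lasts; releasing refills it at a speed-based rate, alongside a debug-drawn predicted arc.
; Route-tagged overlaps fade in splines and switch tracks; a Trace function toggles messages on viewed actors.
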(event `InputAxisKey|MouseY`
  (params (AxisValue :type "Float (single-precision)"))
  ;[1 1 1] マウスの移動量に応じてカメラを回転
  (if (not (`self.isVR`)) :!label _label
    (`SceneComponent.K2_SetRelativeRotation` (`self.Camera`) (`KismetMathLibrary.MakeRotator` 0.0 (`KismetMathLibrary.FClamp` (+ AxisValue (.pitch (`SceneComponent.RelativeRotation` (`self.Camera`)))) -89.0 89.0) (`KismetMathLibrary.FClamp` (+ (.yaw (`SceneComponent.RelativeRotation` (`self.Camera`))) (stale `InputAxisKey|MouseX` AxisValue)) 1.0 179.0)) false false)))

(event `InputAxisKey|MouseX`
  (params (AxisValue :type "Float (single-precision)"))
  ;[1 1 1] マウスの移動量に応じてカメラを回転
  (goto _label))

(event `Key|LeftMouseButton`
  (params (Key :type "Key Structure"))
  (bind _widgetinteraction (`self.WidgetInteraction`))
  ;[1 0.8284 0.2855] ボタン押す設置（林）
  (:`Pressed`
    (`WidgetInteractionComponent.PressPointerKey` _widgetinteraction "LeftMouseButton"))
  (:`Released`
    (`WidgetInteractionComponent.ReleasePointerKey` _widgetinteraction "LeftMouseButton")))

(event `self.ReceiveTick`
  (params (DeltaSeconds :type "Float (single-precision)"))
  (bind _returnvalue (`GameplayStatics.GetWorldDeltaSeconds`))
  (bind _returnvalue_2 (`self.K2_GetActorLocation`))
  (bind _oldlocation (`self.OldLocation`))
  (bind _speed (`self.Speed`))
  (bind _arrow (`self.Arrow`))
  (bind _returnvalue_3 (`SceneComponent.K2_GetComponentLocation` _arrow))
  (bind _returnvalue_4 (* 2.0 (`GameplayStatics.GetWorldDeltaSeconds`)))
  ;[1 1 1] Update
  (`|ExecutionSequence`
    (:`then_0`
      (`/Engine/EditorBlueprintResources/StandardMacros.DoOnce` false
        (:`Completed`
          (`SceneComponent.K2_SetWorldRotation` (`self.DefaultSceneRoot`) (struct :`Yaw` 90.0) false false))))
    (:`then_1`
      ;;[0.1957 1 0.9861] MoveDistanceの値の設定
      (set `self.MoveDistance` (+ (`self.MoveDistance`) (* 100.0 (`self.Speed`) (`self.SpeedRatio`) (`GameplayStatics.GetWorldDeltaSeconds`)))))
    (:`then_2`
      ;;[0.1957 1 0.9861] 位置の更新
      (set `self.OldLocation` (`self.K2_GetActorLocation`))
      (bind _location (`/Game/Data/MySplineActor.GetCurrentLocation` (`|GetArrayItem` (`self.Spline`) (`self.currentSpline`)) (`self.MoveDistance`) false))
      (`self.K2_SetActorLocation` _location))
    (:`then_3`
      ;;[0.1957 1 0.9861] 進行方向に回転
      (if (not (`KismetMathLibrary.EqualExactly_VectorVector` _returnvalue_2 _oldlocation))
        (`self.K2_SetActorRotation` (`KismetMathLibrary.RInterpTo` (`self.K2_GetActorRotation`) (`KismetMathLibrary.FindLookAtRotation` _oldlocation _returnvalue_2) (`GameplayStatics.GetWorldDeltaSeconds`) (`self.TurnAroundTime`)))))
    (:`then_4`
      ;;[0.1957 1 0.9861] speedの設定（下向きに進んでいるときは加速、上向きは減速
      (set `self.SpeedRatio` (`KismetMathLibrary.FClamp` (+ (* (/ (.pitch (`self.K2_GetActorRotation`)) (* -900.0 (`self.SpeedRatioDiv`))) _returnvalue 60.0) (`self.SpeedRatio`) (* _returnvalue -0.4)) 1.0 3.0)))
    (:`then_5`
      (if (`self.canShot`)
        ;;[0.1771 0.9094 0.8765] 連射
        (if (< (`self.FireHold`) 0.0)
          _
          (elif (not (<= (`self.currentBullet`) 0.0))
            (set `self.FireHold` (+ (`self.FireHold`) (`GameplayStatics.GetWorldDeltaSeconds`)))
            (`KismetSystemLibrary.Delay` (`self.ShotInterval`))
            (`|SpawnActorFromClass` "/Game/Data/BallActor.BallActor_C" (`SceneComponent.K2_GetComponentToWorld` (`self.Arrow`)) "Undefined" "OverrideRootScale" null null)
            (`/Engine/EditorBlueprintResources/StandardMacros.DecrementFloat` (`self.currentBullet`)
              (:`  `
                (`TextRenderComponent.K2_SetText` (`self.TextRender`) (`KismetTextLibrary.Conv_IntToText` (`KismetMathLibrary.FTrunc` (`self.currentBullet`)) false true 2 2)) ; 残弾数表示の更新
              ))))))
    (:`then_6`
      ;;[1 1 1] コメント
      (if (< (`self.FireHold`) -0.9)
        (set `self.currentBullet` (`KismetMathLibrary.FMin` (+ (`self.currentBullet`) (* (`self.Speed`) (`GameplayStatics.GetWorldDeltaSeconds`) 1.5)) 30.0))
        (`TextRenderComponent.K2_SetText` (`self.TextRender`) (`KismetTextLibrary.Conv_IntToText` (`KismetMathLibrary.FTrunc` (`self.currentBullet`)) false true 2 2)) ; 残弾数表示の更新
      ))
    (:`then_7`
      (bind _outlaunchvelocity (`GameplayStatics.SuggestProjectileVelocity_CustomArc` _returnvalue_3 (+ _returnvalue_3 (* (`KismetMathLibrary.GetForwardVector` (`SceneComponent.K2_GetComponentRotation` _arrow)) 1000.0)) 0.0 (`self.ArcParam`)))
      (`GameplayStatics.Blueprint_PredictProjectilePath_ByTraceChannel` :`StartPos` _returnvalue_3 :`LaunchVelocity` _outlaunchvelocity :`ProjectileRadius` 10.0 :`TraceChannel` "ECC_Visibility" :`DrawDebugType` "ForOneFrame"))
    (:`then_8`
      ;;[1 1 1] 加速減速
      (if (`self.isAccelerator`)
        (if (not (`self.isBrake`))
          (set `self.Speed` (`KismetMathLibrary.FMin` (+ _speed _returnvalue_4) 9.0)))))
    (:`then_9`
      (if (`self.isBrake`)
        (if (not (`self.isAccelerator`))
          (set `self.Speed` (`KismetMathLibrary.FMax` (- _speed _returnvalue_4) 2.0)))))))

(event `Key|One`
  (params (Key :type "Key Structure"))
  ;[1 1 1] Update
  ;;[0.1957 1 0.9861] 位置の更新
  (:`Pressed`
    (set `self.MoveDistance` 30000.0)))

(event `self.playerOverlapCol.OnComponentBeginOverlap`
  (params (OverlappedComponent :type "PrimitiveComponent Object Reference") (OtherActor :type "Actor Object Reference") (OtherComp :type "PrimitiveComponent Object Reference") (OtherBodyIndex :type Integer) (bFromSweep :type Boolean) (SweepResult :type "HitResult Structure (by ref)"))
  (switch `string` (`KismetStringLibrary.Conv_NameToString` (`|GetArrayItem` (`ActorComponent.ComponentTags` OtherComp)))
    (:`route1`
      (`/Game/Data/MySplineActor.ChangeTransparent` (`|GetArrayItem` (`self.Spline`)) 1.0 1.0))
    (:`route2`
      (`/Game/Data/MySplineActor.ChangeTransparent` (`|GetArrayItem` (`self.Spline`) 1) 1.0 3.0)
      (bind _result (`/Engine/EditorBlueprintResources/StandardMacros.IncrementInt` (`self.currentSpline`) :!label _label_2)
        (:`  `
          (set `self.MoveDistance` 0.0))))
    (:`route3`
      (`/Game/Data/MySplineActor.ChangeTransparent` (`|GetArrayItem` (`self.Spline`) 2) 1.0 3.0)
      (goto _label_2))
    (:`route4`
      (`/Game/Data/MySplineActor.ChangeTransparent` (`|GetArrayItem` (`self.Spline`) 3) 1.0 3.0)
      (goto _label_2))))

(event `InputAction|Fire`
  (params (Key :type "Key Structure"))
  ;[1 1 1] Update
  ;;[1 0.2068 0.7157] 弾の発射
  (:`Pressed`
    (set `self.FireHold` 0.0)
    (`GameplayStatics.PlaySound2D` "/Game/Rin/BGM/SE/shot.shot" 1.0 1.0 0.0 null null))
  (:`Released`
    (set `self.FireHold` -1.0)))

(event `Key|LeftMouseButton`
  (params (Key :type "Key Structure"))
  ;[1 1 1] Update
  ;;[1 1 1] 加速減速
  (:`Pressed`
    (if (`self.canPushButton`)
      (set `self.isAccelerator` true)))
  (:`Released`
    (if (`self.canPushButton`)
      (set `self.isAccelerator` false))))

(event `Key|RightMouseButton`
  (params (Key :type "Key Structure"))
  ;[1 1 1] Update
  ;;[1 1 1] 加速減速
  (:`Pressed`
    (if (`self.canPushButton`)
      (set `self.isBrake` true)))
  (:`Released`
    (if (`self.canPushButton`)
      (set `self.isBrake` false))))

(fn `Trace`
  (bind _camera (`self.Camera`))
  (bind _returnvalue (`SceneComponent.K2_GetComponentLocation` _camera))
  (bind (_outhit _returnvalue_2) (`KismetSystemLibrary.LineTraceSingle` _returnvalue (+ _returnvalue (* (`SceneComponent.GetForwardVector` _camera) 2000)) "TraceTypeQuery1"))
  (if _returnvalue_2
    (bind (_bblockinghit _binitialoverlap _time _distance _location _impactpoint _normal _impactnormal _physmat _hitactor) (`GameplayStatics.BreakHitResult` _outhit))
    (message `/Game/Rin/see.open` _hitactor true)
    (set `self.NewVar_1` _hitactor)
    (else
      (message `/Game/Rin/see.open` (`self.NewVar_1`) false))))

(fn `UserConstructionScript`)