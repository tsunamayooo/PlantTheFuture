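; Player Blueprint that rides a looping spline like a rail shooter, with mouse look outside VR and projectile firing.
; Tick advances the distance along the spline, moves the actor there and smoothly turns it toward its travel direction.
; Pitch feeds a clamped speed ratio that rises downhill and decays otherwise, imitating gravity.
; Fire spawns a shot at the Arrow on press, then Tick spawns delayed repeat projectiles while held.
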(event `InputAxisKey|MouseY`
  (params (AxisValue :type "Float (single-precision)"))
  ;[1 1 1] マウスの移動量に応じてカメラを回転
  (if (not (`self.isVR`)) :!label _label
    (`SceneComponent.K2_SetRelativeRotation` (`self.Camera`) (`KismetMathLibrary.MakeRotator` 0.0 (`KismetMathLibrary.FClamp` (+ AxisValue (.pitch (`SceneComponent.RelativeRotation` (`self.Camera`)))) -89.0 89.0) (`KismetMathLibrary.FClamp` (+ (.yaw (`SceneComponent.RelativeRotation` (`self.Camera`))) (stale `InputAxisKey|MouseX` AxisValue)) 1.0 179.0)) false false)))

(event `InputAxisKey|MouseX`
  (params (AxisValue :type "Float (single-precision)"))
  ;[1 1 1] マウスの移動量に応じてカメラを回転
  (goto _label))

(event `self.ReceiveTick`
  (params (DeltaSeconds :type "Float (single-precision)"))
  ;[1 1 1] Update
  (`|ExecutionSequence`
    (:`then_0`
      ;;[0.1957 1 0.9861] MoveDistanceの値の設定
      (set `self.MoveDistance` (+ (`self.MoveDistance`) (* (`GameplayStatics.GetWorldDeltaSeconds`) 100.0 (`self.Speed`) (`self.SpeedRatio`)))))
    (:`then_1`
      ;;[0.1957 1 0.9861] 位置の更新
      (set `self.OldLocation` (`self.K2_GetActorLocation`))
      (bind _location (`/Game/Data/MySplineActor.GetCurrentLocation` (`self.Spline`) (`self.MoveDistance`) true))
      (`self.K2_SetActorLocation` _location))
    (:`then_2`
      ;;[0.1957 1 0.9861] 進行方向に回転
      (`self.K2_SetActorRotation` (`KismetMathLibrary.RInterpTo` (`self.K2_GetActorRotation`) (`KismetMathLibrary.FindLookAtRotation` (`self.OldLocation`) (`self.K2_GetActorLocation`)) (`GameplayStatics.GetWorldDeltaSeconds`) (`self.TurnAroundTime`))))
    (:`then_3`
      ;;[0.1957 1 0.9861] speedの設定（下向きに進んでいるときは加速、上向きは減速
      (set `self.SpeedRatio` (`KismetMathLibrary.FClamp` (+ (/ (.pitch (`self.K2_GetActorRotation`)) (* -900.0 (`self.SpeedRatioDiv`))) (* (`GameplayStatics.GetWorldDeltaSeconds`) -0.4) (`self.SpeedRatio`)) 1.0 2.5)))
    (:`then_4`
      ;;[0.1771 0.9094 0.8765] 連射
      (if (not (< (`self.FireHold`) 0.0))
        (set `self.FireHold` (+ (`self.FireHold`) (`GameplayStatics.GetWorldDeltaSeconds`)))
        (`KismetSystemLibrary.Delay` (`self.ShotInterval`))
        (`|SpawnActorFromClass` "/Game/Data/fura/FirstPersonProjectile/FirstPersonProjectile.FirstPersonProjectile_C" (`SceneComponent.K2_GetComponentToWorld` (`self.Arrow`)) "Undefined" "OverrideRootScale" null null)))))

(event `InputAction|Fire`
  (params (Key :type "Key Structure"))
  ;[1 1 1] Update
  ;;[1 0.2068 0.7157] 弾の発射
  (:`Pressed`
    (set `self.FireHold` 0.0)
    (`|SpawnActorFromClass` "/Game/Data/fura/FirstPersonProjectile/FirstPersonProjectile.FirstPersonProjectile_C" (`SceneComponent.K2_GetComponentToWorld` (`self.Arrow`)) "Undefined" "OverrideRootScale" null null))
  (:`Released`
    (set `self.FireHold` -1.0)))

(fn `UserConstructionScript`)